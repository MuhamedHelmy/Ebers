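; BP_MusicBall is an actor whose ball mesh moves toward the BP_Cage actors when play begins.
; A timeline starts on BeginPlay and, each update, finds all cages and teleports the mesh toward each in turn, lerping from its current location by the timeline's alpha.
; The box component's overlap event only prints a debug string.
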(event OnComponentBeginOverlap(Box_MusicBall)
  (params (OverlappedComponent :type Primitive%20Component%20Object%20Reference) (OtherActor :type Actor%20Object%20Reference) (OtherComp :type Primitive%20Component%20Object%20Reference) (OtherBodyIndex :type Integer) (bFromSweep :type Boolean) (SweepResult :type Hit%20Result%20Structure%20%28by%20ref%29))
  (Development|PrintString "MusicBall"))

(event EventBeginPlay
  (bind _newtrack_0 (Timeline|Timeline_0 PlayFromStart)
    (:Update
      (bind _outactors (Actor|GetAllActorsOfClass "/Game/Blueprints/BP_Cage.BP_Cage_C"))
      (for _array_element _outactors
        (Transformation|SetWorldLocation (Variables|Default|GetSM_MyMusicBall) (Math|Vector|Lerp(Vector) (Transformation|GetWorldLocation (Variables|Default|GetSM_MyMusicBall)) (Transformation|GetActorLocation _array_element) _newtrack_0) false true)))))

(event Collision|EventActorBeginOverlap
  (params (OtherActor :type Actor%20Object%20Reference)))

(event EventTick
  (params (DeltaSeconds :type Float%20%28single-precision%29)))

(fn ConstructionScript)
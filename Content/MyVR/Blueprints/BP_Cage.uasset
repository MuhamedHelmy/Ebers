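; BP_Cage is a destructible cage actor in the MyVR project that takes damage from BP_MusicBall actors.
; When an actor overlaps Box_Cage, it prints a debug string and checks whether that actor's class is exactly BP_MusicBall.
; A matching ball is destroyed and lowers the cage's Health by a fixed amount, and the cage destroys itself once Health reaches zero or below.
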(event OnComponentBeginOverlap(Box_Cage)
  (params (OverlappedComponent :type Primitive%20Component%20Object%20Reference) (OtherActor :type Actor%20Object%20Reference) (OtherComp :type Primitive%20Component%20Object%20Reference) (OtherBodyIndex :type Integer) (bFromSweep :type Boolean) (SweepResult :type Hit%20Result%20Structure%20%28by%20ref%29))
  (Development|PrintString "Cage")
  (if (== (Utilities|GetClass OtherActor) "/Game/Blueprints/BP_MusicBall.BP_MusicBall_C")
    (Actor|DestroyActor OtherActor)
    (Variables|Default|SetHealth (- (Variables|Default|GetHealth) 10))
    (if (<= (Variables|Default|GetHealth) 0)
      (Actor|DestroyActor self))))

(event EventBeginPlay)

(event Collision|EventActorBeginOverlap
  (params (OtherActor :type Actor%20Object%20Reference)))

(event EventTick
  (params (DeltaSeconds :type Float%20%28single-precision%29)))

(fn ConstructionScript)
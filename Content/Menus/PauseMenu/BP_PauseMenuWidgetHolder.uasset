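; Actor that holds the in-world pause menu widget component and links it to the current minigame's manager.
; On BeginPlay it casts the widget to WBP_PauseMenu and hands it a reference to itself.
; It then searches the level for a drum, dance or mimic game manager, in that order, and assigns the first valid one as the menu's GameManagerRef.
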(event EventBeginPlay
  (bind _aswbp_pause_menu (Utilities|Casting|CastToWBP_PauseMenu (UserInterface|GetWidget (Variables|Default|GetWidget))))
  (Variables|/Game/Menus/PauseMenu/WBP_PauseMenu.WBP_PauseMenu_C|SetPauseMenuRef _aswbp_pause_menu self)
  (bind _returnvalue (Actor|GetActorOfClass "/Script/Ebers.DrumManger"))
  (Utilities|IsValid _returnvalue
    (:Is%20Valid
      (Variables|/Game/Menus/PauseMenu/WBP_PauseMenu.WBP_PauseMenu_C|SetGameManagerRef _aswbp_pause_menu _returnvalue))
    (:Is%20Not%20Valid
      (bind _returnvalue_2 (Actor|GetActorOfClass "/Game/Blueprints/DanceBP/BP_DanceGameManager.BP_DanceGameManager_C"))
      (Utilities|IsValid _returnvalue_2
        (:Is%20Valid
          (Variables|/Game/Menus/PauseMenu/WBP_PauseMenu.WBP_PauseMenu_C|SetGameManagerRef _aswbp_pause_menu _returnvalue_2))
        (:Is%20Not%20Valid
          (bind _returnvalue_3 (Actor|GetActorOfClass "/Game/Blueprints/MimicBP/WallBP/Mangers/MyMimicGameManager.MyMimicGameManager_C"))
          (Utilities|IsValid _returnvalue_3
            (:Is%20Valid
              (Variables|/Game/Menus/PauseMenu/WBP_PauseMenu.WBP_PauseMenu_C|SetGameManagerRef _aswbp_pause_menu _returnvalue_3))))))))

(event Collision|EventActorBeginOverlap
  (params (OtherActor :type Actor%20Object%20Reference)))

(event EventTick
  (params (DeltaSeconds :type Float%20%28single-precision%29)))

(fn ConstructionScript)
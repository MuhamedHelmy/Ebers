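; BP_DrumManger is the manager for the drum game, handling its end screen and pause menu.
; On BeginPlay it registers itself as GameManager on the BP_EbersPlayer pawn.
; Tick polls EndGame, then once spawns the win/lose widget holder actor and destroys the score holder, latched by EndTick.
; ShowPauseMenu toggles a spawned pause menu holder and the Pause flag until the game ends.
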(event EventBeginPlay
  (bind _asbp_ebers_player (Utilities|Casting|CastToBP_EbersPlayer (Game|Player|GetPlayerPawn 0)))
  (Variables|/Game/Blueprints/PlayerBP/BP_EbersPlayer.BP_EbersPlayer_C|SetGameManager _asbp_ebers_player self))

(event Collision|EventActorBeginOverlap
  (params (OtherActor :type Actor%20Object%20Reference)))

(event EventTick
  (params (DeltaSeconds :type Float%20%28single-precision%29))
  (if (not (Variables|Default|GetEndTick))
    (if (Variables|Default|GetbEndGame)
      (Game|SpawnActorfromClass "/Game/Menus/WinLoseMenu/BP_WinLoseMenuWidgetHolder.BP_WinLoseMenuWidgetHolder_C" (Math|Transform|MakeTransform "750.000000,-5.000000,351.000000" "0, 0, 0" "1,1,1") "Undefined" 0 0)
      (Variables|Default|SetEndTick true)
      (Actor|DestroyActor (Variables|Default|GetScoreHolderRef))
      (Development|PrintString "mmmmmmmmmmmmmm"))))

(event Input|ActionEvents|InputActionShowPauseMenu
  (params (Key :type Key%20Structure :default "None"))
  (:Pressed
    (if (not (Variables|Default|GetbEndGame))
      (if (not (Variables|Default|GetbPause))
        (bind _returnvalue (Game|SpawnActorfromClass "/Game/Menus/PauseMenu/BP_PauseMenuWidgetHolder.BP_PauseMenuWidgetHolder_C" (Math|Transform|MakeTransform "528.000000,-5.000000,291.000000" "0, 0, 0" "1,1,1") "Undefined" 0 0))
        (Variables|Default|SetPauseMenuRef _returnvalue)
        ;[1 1 1] in code DanceManager
        (Variables|Default|SetbPause true)
        (else
          (Actor|DestroyActor (Variables|Default|GetPauseMenuRef))
          (Variables|Default|SetbPause false))))))

(fn ConstructionScript)
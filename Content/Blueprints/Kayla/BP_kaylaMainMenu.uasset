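; BP_kaylaMainMenu is a Kayla actor, named for the main menu, that plays a timed animation sequence on its skeletal mesh.
; BeginPlay sets wave, point and end flags at three-second intervals.
; Tick uses the first active flag to raise BBSKayla on AnimBp_Kayla toward that phase's threshold, then clears the flag.
; The increments are fixed per frame, so blend speed depends on frame rate.
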(event EventBeginPlay
  (Utilities|FlowControl|Delay 3.0)
  (Variables|Default|SetStartWave true)
  (Utilities|FlowControl|Delay 3.0)
  (Variables|Default|SetStartPoint true)
  (Utilities|FlowControl|Delay 3.0)
  (Variables|Default|SetEndAnim true))

(event Collision|EventActorBeginOverlap
  (params (OtherActor :type Actor%20Object%20Reference)))

(event EventTick
  (params (DeltaSeconds :type Float%20%28single-precision%29))
  (if (Variables|Default|GetStartWave)
    (bind _asanim_bp_kayla (Utilities|Casting|CastToAnimBp_Kayla (Components|SkeletalMesh|GetAnimInstance (Variables|Default|GetSkeletalMesh))))
    (Variables|/Game/Art/Characters/kayla/Animation/AnimBp_Kayla.AnimBp_Kayla_C|SetbBS_Kayla _asanim_bp_kayla (+ (Variables|/Game/Art/Characters/kayla/Animation/AnimBp_Kayla.AnimBp_Kayla_C|GetbBS_Kayla _asanim_bp_kayla) 1.0))
    (if (>= (Variables|/Game/Art/Characters/kayla/Animation/AnimBp_Kayla.AnimBp_Kayla_C|GetbBS_Kayla _asanim_bp_kayla) 5e+01)
      (Variables|Default|SetStartWave false))
    (elif (Variables|Default|GetStartPoint)
      (bind _asanim_bp_kayla_2 (Utilities|Casting|CastToAnimBp_Kayla (Components|SkeletalMesh|GetAnimInstance (Variables|Default|GetSkeletalMesh))))
      (Variables|/Game/Art/Characters/kayla/Animation/AnimBp_Kayla.AnimBp_Kayla_C|SetbBS_Kayla _asanim_bp_kayla_2 (+ (Variables|/Game/Art/Characters/kayla/Animation/AnimBp_Kayla.AnimBp_Kayla_C|GetbBS_Kayla _asanim_bp_kayla_2) 0.5))
      (if (>= (Variables|/Game/Art/Characters/kayla/Animation/AnimBp_Kayla.AnimBp_Kayla_C|GetbBS_Kayla _asanim_bp_kayla_2) 75.0)
        (Variables|Default|SetStartPoint false))
      (elif (Variables|Default|GetEndAnim)
        (bind _asanim_bp_kayla_3 (Utilities|Casting|CastToAnimBp_Kayla (Components|SkeletalMesh|GetAnimInstance (Variables|Default|GetSkeletalMesh))))
        (Variables|/Game/Art/Characters/kayla/Animation/AnimBp_Kayla.AnimBp_Kayla_C|SetbBS_Kayla _asanim_bp_kayla_3 (+ (Variables|/Game/Art/Characters/kayla/Animation/AnimBp_Kayla.AnimBp_Kayla_C|GetbBS_Kayla _asanim_bp_kayla_3) 0.5))
        (if (>= (Variables|/Game/Art/Characters/kayla/Animation/AnimBp_Kayla.AnimBp_Kayla_C|GetbBS_Kayla _asanim_bp_kayla_3) 1e+02)
          (Variables|Default|SetEndAnim false))))))

(fn ConstructionScript)
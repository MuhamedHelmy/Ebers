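; Dance game manager that drives the score readout on a laser score widget holder.
; Each Tick, while the game runs, it compares rounded PointsScore to SavedScore and rewrites the score text only on a change.
; Once EndGame is set, it shows the score as a rounded percentage of TotalScore and latches EndTick to stop further updates.
; The graph only reads PointsScore, TotalScore and EndGame, and never sets them.
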(event EventBeginPlay)

(event Collision|EventActorBeginOverlap
  (params (OtherActor :type Actor%20Object%20Reference)))

(event EventTick
  (params (DeltaSeconds :type Float%20%28single-precision%29))
  (bind _pointsscore (Variables|Default|GetpointsScore))
  (bind _returnvalue (Class|KismetMathLibrary|Round64 _pointsscore))
  (if (not (Variables|Default|GetEndTick))
    (if (Variables|Default|GetEndGame)
      (bind _asbp_laser_score_widget_hoder (Utilities|Casting|CastToBP_LaserScoreWidgetHoder (Variables|Default|GetLaserScore)))
      (Rendering|Components|TextRender|SetText (Variables|/Game/BP_LaserScoreWidgetHoder.BP_LaserScoreWidgetHoder_C|GetTxt%20Score _asbp_laser_score_widget_hoder) (Utilities|Text|ToText(String) (Utilities|String|Append "Score: " (Utilities|String|ToString(Text) (Utilities|Text|ToText(String) (Class|KismetMathLibrary|Round64 (* 100 (/ (Variables|Default|GetpointsScore) (Variables|Default|GettotalScore)))))) "%")))
      (Variables|Default|SetEndTick true)
      (elif (!= (Class|KismetMathLibrary|Round64 (Variables|Default|GetSavedScore)) _returnvalue)
        (bind _asbp_laser_score_widget_hoder_2 (Utilities|Casting|CastToBP_LaserScoreWidgetHoder (Variables|Default|GetLaserScore)))
        (Variables|Default|SetSavedScore _pointsscore)
        (Rendering|Components|TextRender|SetText (Variables|/Game/BP_LaserScoreWidgetHoder.BP_LaserScoreWidgetHoder_C|GetTxt%20Score _asbp_laser_score_widget_hoder_2) (Utilities|Text|ToText(String) (Utilities|String|Append "Score: " (Utilities|String|ToString(Text) (Utilities|Text|ToText(String) _returnvalue)))))))))

(fn ConstructionScript)
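; VR player pawn that aims a laser at dance enemies and operates UI through widget interaction.
; Unless paused, each tick it line-traces from the laser position, flagging any BP_DanceEnemy hit.
; A hit marker follows the widget hit while a spline mesh is stretched between spline points as the beam.
; It also sets a floor tracking origin, turns UIPress into pointer clicks and drives hand animation from trigger axes; ExecuteGrab is empty.
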(event EventBeginPlay
  ;[1 1 1] Set Tracking Origin as Floor
  (Class|HeadMountedDisplayFunctionLibrary|SetTrackingOrigin "Floor"))

(event EventTick
  (params (DeltaSeconds :type Float%20%28single-precision%29))
  (bind _laserposition (Variables|Default|GetLaserPosition))
  (bind _widgetinteraction (Variables|Default|GetWidgetInteraction))
  (bind _returnvalue (Class|WidgetInteractionComponent|GetLastHitResult _widgetinteraction))
  (bind _returnvalue_2 (Transformation|GetWorldLocation _laserposition))
  (Utilities|FlowControl|Sequence
    (:then_0
      (if (not (Variables|Default|GetPausePlayer))
        (bind (_outhit _returnvalue_3) (Collision|LineTraceForObjects _returnvalue_2 (+ _returnvalue_2 (* (Math|Vector|GetForwardVector (Transformation|GetWorldRotation _laserposition)) 4e+02)) (Variables|Default|GetObject%20Types) false 0 "None"))
        (Utilities|FlowControl|Sequence
          (:then_0
            (if _returnvalue_3
              (bind _asbp_dance_enemy (Utilities|Casting|CastToBP_DanceEnemy (.HitActor (Collision|BreakHitResult _outhit)))
                (:then
                  (Variables|/Game/Blueprints/DanceBP/BP_DanceEnemy.BP_DanceEnemy_C|SetbHitSphere _asbp_dance_enemy true)
                  (Variables|Default|SetIsEnemyCast true))
                (:CastFailed
                  (Variables|Default|SetIsEnemyCast false)))))
          (:then_1
            (if (not _returnvalue_3)
              (Variables|Default|SetIsInCurve false))))))
    (:then_1
      ;[1 1 1] widget Spline
      (if (.bblockinghit _returnvalue)
        (Development|SetHiddeninGame (Variables|Default|GetInteractionHitSphere) false false)
        (Transformation|SetWorldLocation (Variables|Default|GetInteractionHitSphere) (.location _returnvalue) false false)
        (Spline|SetLocationatSplinePoint (Variables|Default|GetSpline) 1 (.location _returnvalue) "World" true)
        (CallFunction|UpdateInteractionBeam (Variables|Default|GetSpline1) (Variables|Default|GetSplineMesh))
        (else
          (Development|SetHiddeninGame (Variables|Default|GetInteractionHitSphere) true false)
          (Development|SetHiddeninGame (Variables|Default|GetSplineMesh) true false))))))

(event Input|ActionEvents|InputActionUIPress
  (params (Key :type Key%20Structure :default "None"))
  (bind _widgetinteraction (Variables|Default|GetWidgetInteraction))
  ;[1 1 1] Widget Interaction
  (:Pressed
    (Class|WidgetInteractionComponent|PressPointerKey _widgetinteraction "LeftMouseButton"))
  (:Released
    (Class|WidgetInteractionComponent|ReleasePointerKey _widgetinteraction "LeftMouseButton")))

(event Input|AxisEvents|InputAxisTriggerAxisLeft
  (params (AxisValue :type Float%20%28single-precision%29))
  ;[1 1 1] VRHandAnimation
  (bind _asabp_vrhand (Utilities|Casting|CastToABP_VRHand (Components|SkeletalMesh|GetAnimInstance (Variables|Default|GetHandMesh_Left))))
  (Variables|/Game/hand/ABP_VRHand.ABP_VRHand_C|SetMySpeedAnim _asabp_vrhand AxisValue))

(event Input|AxisEvents|InputAxisTriggerAxisRight
  (params (AxisValue :type Float%20%28single-precision%29))
  ;[1 1 1] VRHandAnimation
  (bind _asabp_vrhand (Utilities|Casting|CastToABP_VRHand (Components|SkeletalMesh|GetAnimInstance (Variables|Default|GetHandMesh_Right))))
  (Variables|/Game/hand/ABP_VRHand.ABP_VRHand_C|SetMySpeedAnim _asabp_vrhand AxisValue))

(fn ConstructionScript)

(fn UpdateInteractionBeam
  (params (MySpline :type Spline%20Component%20Object%20Reference) (MySplineMesh :type Spline%20Mesh%20Component%20Object%20Reference))
  (bind (_location _tangent) (Spline|GetLocationandTangentatSplinePoint MySpline 0 "World"))
  (bind (_location_2 _tangent_2) (Spline|GetLocationandTangentatSplinePoint MySpline 1 "World"))
  (Development|SetHiddeninGame MySplineMesh false false)
  (SplineMesh|SetStartandEnd MySplineMesh _location _tangent _location_2 _tangent_2 true :!class /Script/Engine.SplineMeshComponent))

(fn ExecuteGrab
  (params (MotionController :type Scene%20Component%20Object%20Reference))
  (return 0))
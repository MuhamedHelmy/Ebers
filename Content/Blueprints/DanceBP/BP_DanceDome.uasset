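; BP_DanceDome is a dome actor that loses health when BP_EbersPlayer overlaps its Box component.
; Each such overlap lowers DomeHealth by one and prints the new value.
; An overlap that finds health already at zero or below prints "lose" and destroys the actor.
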(event OnComponentBeginOverlap(Box)
  (params (OverlappedComponent :type Primitive%20Component%20Object%20Reference) (OtherActor :type Actor%20Object%20Reference) (OtherComp :type Primitive%20Component%20Object%20Reference) (OtherBodyIndex :type Integer) (bFromSweep :type Boolean) (SweepResult :type Hit%20Result%20Structure%20%28by%20ref%29))
  (if (== (Utilities|GetClass OtherActor) "/Game/Blueprints/PlayerBP/BP_EbersPlayer.BP_EbersPlayer_C")
    (if (> (Variables|Default|GetDomeHealth) 0.0)
      (bind _output_get (Variables|Default|SetDomeHealth (- (Variables|Default|GetDomeHealth) 1.0)))
      (Development|PrintString (Utilities|String|Append "Dome Health: " (Utilities|String|ToString(Float) _output_get)))
      (else
        (Development|PrintString "lose")
        (Actor|DestroyActor self)))))

(event EventBeginPlay)

(event Collision|EventActorBeginOverlap
  (params (OtherActor :type Actor%20Object%20Reference)))

(event EventTick
  (params (DeltaSeconds :type Float%20%28single-precision%29)))

(fn ConstructionScript)
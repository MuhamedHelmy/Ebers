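; BP_DanceGameManager runs pause and end-of-game flow for the dance game, registering itself with BP_EbersPlayer on BeginPlay.
; ShowPauseMenu spawns or destroys a pause menu widget-holder actor, syncing the pause flags and hiding or showing the player's two spline meshes.
; Tick polls EndGame and, once, spawns the win/lose menu holder, hides those meshes and destroys the LaserScore actor.
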(event EventBeginPlay
  (Input|EnableInput (Game|GetPlayerController 0))
  (bind _asbp_ebers_player (Utilities|Casting|CastToBP_EbersPlayer (Game|Player|GetPlayerPawn 0)))
  (Variables|/Game/Blueprints/PlayerBP/BP_EbersPlayer.BP_EbersPlayer_C|SetGameManager _asbp_ebers_player self))

(event EventTick
  (params (DeltaSeconds :type Float%20%28single-precision%29))
  (if (not (Variables|Default|GetEndTick))
    (if (Variables|Default|GetEndGame)
      (Game|SpawnActorfromClass "/Game/Menus/WinLoseMenu/BP_WinLoseMenuWidgetHolder.BP_WinLoseMenuWidgetHolder_C" (Math|Transform|MakeTransform "750.000000,-5.000000,291.000000" "0, 0, 0" "1,1,1") "Undefined" 0 0)
      (Variables|Default|SetEndTick true)
      (Development|PrintString "eeeeeend")
      (bind _asbp_ebers_player (Utilities|Casting|CastToBP_EbersPlayer (Game|Player|GetPlayerPawn 0)))
      (Development|SetHiddeninGame (Variables|/Game/Blueprints/PlayerBP/BP_EbersPlayer.BP_EbersPlayer_C|GetSplineMesh1 _asbp_ebers_player) true false)
      (Development|SetHiddeninGame (Variables|/Game/Blueprints/PlayerBP/BP_EbersPlayer.BP_EbersPlayer_C|GetSplineMesh2 _asbp_ebers_player) true false)
      (Actor|DestroyActor (Variables|Default|GetLaserScore)))))

(event Input|ActionEvents|InputActionShowPauseMenu
  (params (Key :type Key%20Structure))
  (:Pressed
    (if (not (Variables|Default|GetEndGame))
      (if (not (Variables|Default|GetbPause))
        (bind _returnvalue (Game|SpawnActorfromClass "/Game/Menus/PauseMenu/BP_PauseMenuWidgetHolder.BP_PauseMenuWidgetHolder_C" (Math|Transform|MakeTransform "528.000000,-5.000000,291.000000" "0, 0, 0" "1,1,1") "Undefined" 0 0))
        (Variables|Default|SetPauseMenuRef _returnvalue)
        ;[1 1 1] in code DanceManager
        (Variables|Default|SetbPause true)
        (bind _asbp_ebers_player (Utilities|Casting|CastToBP_EbersPlayer (Game|Player|GetPlayerPawn 0)))
        ;[1 1 1] In EbersPlayerBP
        (Variables|/Game/Blueprints/PlayerBP/BP_EbersPlayer.BP_EbersPlayer_C|SetPausePlayer _asbp_ebers_player true)
        (Development|SetHiddeninGame (Variables|/Game/Blueprints/PlayerBP/BP_EbersPlayer.BP_EbersPlayer_C|GetSplineMesh1 _asbp_ebers_player) true false)
        (Development|SetHiddeninGame (Variables|/Game/Blueprints/PlayerBP/BP_EbersPlayer.BP_EbersPlayer_C|GetSplineMesh2 _asbp_ebers_player) true false)
        (else
          (Actor|DestroyActor (Variables|Default|GetPauseMenuRef))
          (Variables|Default|SetbPause false)
          (bind _asbp_ebers_player_2 (Utilities|Casting|CastToBP_EbersPlayer (Game|Player|GetPlayerPawn 0)))
          (Variables|/Game/Blueprints/PlayerBP/BP_EbersPlayer.BP_EbersPlayer_C|SetPausePlayer _asbp_ebers_player_2 false)
          (Development|SetHiddeninGame (Variables|/Game/Blueprints/PlayerBP/BP_EbersPlayer.BP_EbersPlayer_C|GetSplineMesh1 _asbp_ebers_player_2) false false)
          (Development|SetHiddeninGame (Variables|/Game/Blueprints/PlayerBP/BP_EbersPlayer.BP_EbersPlayer_C|GetSplineMesh2 _asbp_ebers_player_2) false false))))))

(fn ConstructionScript)
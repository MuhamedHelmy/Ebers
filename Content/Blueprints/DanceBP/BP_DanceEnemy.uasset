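; BP_DanceEnemy is an enemy actor that can be destroyed once hit, apparently within a dance minigame.
; Each Tick it polls HitSphere, destroying itself and setting the player's IsInCurve when CanAttack is true.
; A hit without CanAttack instead clears IsInCurve and HitSphere if the player's IsEnemyCast is set.
; Health, manager-array and attack-order message nodes remain disconnected and never run.
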(event EventBeginPlay)

(event Collision|EventActorBeginOverlap
  (params (OtherActor :type Actor%20Object%20Reference)))

(event EventTick
  (params (DeltaSeconds :type Float%20%28single-precision%29))
  (bind _returnvalue (Game|Player|GetPlayerPawn 0))
  (if (Variables|Default|GetbHitSphere)
    (if (Variables|Default|GetcanAttack)
      (Actor|DestroyActor self)
      (Variables|Default|SetDestroyedDone true)
      (bind _asbp_ebers_player (Utilities|Casting|CastToBP_EbersPlayer _returnvalue))
      (Variables|/Script/Ebers.EbersPlayer|SetIsInCurve _asbp_ebers_player true)
      (else
        (bind _asbp_ebers_player_2 (Utilities|Casting|CastToBP_EbersPlayer _returnvalue))
        (if (Variables|/Game/Blueprints/PlayerBP/BP_EbersPlayer.BP_EbersPlayer_C|GetIsEnemyCast _asbp_ebers_player_2)
          (Variables|/Script/Ebers.EbersPlayer|SetIsInCurve _asbp_ebers_player_2 false)
          (Variables|Default|SetbHitSphere false))))))

(fn ConstructionScript)
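; BP_EbersPlayer is a player blueprint, apparently for VR, that points at and clicks UI widgets.
; BeginPlay stores the camera and sets floor tracking origin; UIPress drives the WidgetInteraction left-mouse pointer.
; Each tick, a blocking widget hit shows a sphere there, moves the right shoulder spline's end to it and unhides that spline.
; Without a hit only the sphere is hidden.
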(event EventBeginPlay
  ;[1 1 1] Set Tracking Origin as Floor
  (Utilities|FlowControl|Sequence
    (:then_0
      (Variables|Default|Setmycamera (Variables|Default|GetCamera)))
    (:then_1
      (Class|HeadMountedDisplayFunctionLibrary|SetTrackingOrigin "Floor"))))

(event EventTick
  (params (DeltaSeconds :type Float%20%28single-precision%29))
  (bind _widgetinteraction (Variables|Default|GetWidgetInteraction))
  (bind _interactionhitsphere (Variables|Default|GetInteractionHitSphere))
  (bind _returnvalue (Class|WidgetInteractionComponent|GetLastHitResult _widgetinteraction))
  (Utilities|FlowControl|Sequence
    (:then_0
      ;[1 1 1] widget Spline
      (if (.bblockinghit _returnvalue)
        (Development|SetHiddeninGame (Variables|Default|GetInteractionHitSphere) false false)
        (Transformation|SetWorldLocation _interactionhitsphere (.location _returnvalue) false false)
        (Spline|SetLocationatSplinePoint (Variables|Default|GetRightShoulderSpline) 1 (.location _returnvalue) "World" true)
        (CallFunction|UpdateInteractionBeam)
        (else
          (Development|SetHiddeninGame (Variables|Default|GetInteractionHitSphere) true false)
          (Development|SetHiddeninGame _interactionhitsphere true false))))))

(event Input|ActionEvents|InputActionUIPress
  (params (Key :type Key%20Structure))
  (bind _widgetinteraction (Variables|Default|GetWidgetInteraction))
  ;[1 1 1] Widget Interaction
  (:Pressed
    (Class|WidgetInteractionComponent|PressPointerKey _widgetinteraction "LeftMouseButton"))
  (:Released
    (Class|WidgetInteractionComponent|ReleasePointerKey _widgetinteraction "LeftMouseButton")))

(fn ConstructionScript)

(fn UpdateInteractionBeam
  (Development|SetHiddeninGame (Variables|Default|GetRightShoulderSpline) false false))